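; Player character for a voxel-world game, tagged as the player on BeginPlay and carrying heavy world-generation debug output.
; Tick counts down an action delay, notifies the line-traced actor that it is visible, and prints location, region and terrain-shaper values.
; For chunk hits, it nudges the impact point along the ray to identify and print the block.
; Head submersion events switch the underwater post-process material and walk, jump and step settings.
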(event EventTick
  (params (DeltaSeconds :type Float%20%28single-precision%29))
  (CallFunction|ShowLocationDebug)
  (CallFunction|ShowTerrainGenDebug)
  (if (not false)
    (Variables|Default|SetActionDelay (Math|Float|Clamp(Float) (- (Variables|Default|GetActionDelay) DeltaSeconds)))
    (bind _hitresult (Class|PlayerCharacter|VisibilityLineTrace))
    (Class|InteractableActor|OnVisiblebyCharacter(Message) (.HitActor (Collision|BreakHitResult _hitresult)) self _hitresult)
    (bind _asachunk_bp (Utilities|Casting|CastToAChunk_BP (.HitActor (Collision|BreakHitResult _hitresult))))
    (Development|PrintString (Utilities|String|Append "Hit chunk: " (Utilities|GetDisplayName _asachunk_bp) " | Gen stage: " (Utilities|String|EnumtoString (Class|Chunk|GetGenStage _asachunk_bp)) " | border chunk: " (Utilities|String|ToString(Boolean) (Class|Chunk|IsBorderChunk _asachunk_bp)) " 
 Local Pos: " (Utilities|String|ToString(Integer) (Class|ChunkUtilityLib|WorldLocationtoLocalBlockPos (+ (.Location (Collision|BreakHitResult _hitresult)) (* (Math|Rotator|GetRotationXVector (Math|Rotator|FindLookatRotation (.TraceStart (Collision|BreakHitResult _hitresult)) (.TraceEnd (Collision|BreakHitResult _hitresult)))) 3.0)))) " | Hit Block: " (Utilities|String|ToString(Name) (.DisplayName (Utilities|Struct|BreakBlockData (Class|BlockDataSubsystem|GetBlockDataBP (|BlockDataSubsystem) (Class|KismetMathLibrary|ToInt64(Integer) (Utilities|Struct|BreakBlockState (Class|Chunk|GetBlockatLocalPosition _asachunk_bp (Class|ChunkUtilityLib|WorldLocationtoLocalBlockPos (+ (.Location (Collision|BreakHitResult _hitresult)) (* (Math|Rotator|GetRotationXVector (Math|Rotator|FindLookatRotation (.TraceStart (Collision|BreakHitResult _hitresult)) (.TraceEnd (Collision|BreakHitResult _hitresult)))) 3.0))))))))))) true false "(R=0.547314,G=1.000000,B=0.114522,A=1.000000)" 2.0 "HitChunk")))

(event EventBeginPlay
  (bind _charactergameplaytags (Variables|Default|GetCharacterGameplayTags))
  (GameplayTags|AddGameplayTag _charactergameplaytags "(TagName=\"Terrestre.Character.Player\")" :!class /Script/GameplayTags.BlueprintGameplayTagLibrary)
  (Development|PrintString (GameplayTags|GetDebugStringfromGameplayTagContainer _charactergameplaytags)))

(event EventOnHeadSubmerged
  (bind _charactermovement (Variables|Character|GetCharacterMovement))
  (Variables|/Script/Engine.CameraComponent|SetPostProcessSettings (Variables|Default|GetCamera) (Utilities|Struct|MakePostProcessSettings (Utilities|Struct|MakeWeightedBlendables (Utilities|Array|MakeArray (Utilities|Struct|MakeWeightedBlendable 1.0 "/Game/Core/World/Materials/Water/UnderwaterPP_M.UnderwaterPP_M")))))
  (Variables|/Script/Engine.CharacterMovementComponent|SetMaxWalkSpeed _charactermovement 2e+02)
  (Variables|/Script/Engine.CharacterMovementComponent|SetJumpZVelocity _charactermovement 3e+02)
  (Variables|/Script/Engine.CharacterMovementComponent|SetMaxStepHeight _charactermovement 1e+02))

(event EventOnHeadAboveLiquid
  (bind _charactermovement (Variables|Character|GetCharacterMovement))
  (Variables|/Script/Engine.CameraComponent|SetPostProcessSettings (Variables|Default|GetCamera) (Utilities|Struct|MakePostProcessSettings (Utilities|Struct|MakeWeightedBlendables (Utilities|Array|MakeArray ""))))
  (Variables|/Script/Engine.CharacterMovementComponent|SetMaxWalkSpeed _charactermovement 5.5e+02)
  (Variables|/Script/Engine.CharacterMovementComponent|SetJumpZVelocity _charactermovement 5.2e+02)
  (Variables|/Script/Engine.CharacterMovementComponent|SetMaxStepHeight _charactermovement 5e+01))

(fn ConstructionScript)

(fn ShowTerrainGenDebug
  (bind _returnvalue (Transformation|GetActorLocation))
  (bind _returnvalue_2 (Transformation|GetActorLocation))
  (bind _returnvalue_3 (Transformation|GetActorLocation))
  (bind _returnvalue_4 (Subsystems|GetWorldGenSubsystem))
  (bind _returnvalue_5 (Class|WorldGenSubsystem|GetTerrainShaper _returnvalue_4))
  (bind _returnvalue_6 (Class|TerrainShaper|GetInitialDensityatXYZBP _returnvalue_5 (.x _returnvalue_2) (.y _returnvalue_2) (.z _returnvalue_2)))
  (Utilities|FlowControl|Sequence
    (:then_0
      (Development|PrintString (Class|KismetStringLibrary|BuildStringDouble "Cont: " "" (Class|TerrainShaper|GetContinentalnessatXYBP _returnvalue_5 (.x _returnvalue) (.y _returnvalue))) true false "(R=1.000000,G=0.008023,B=0.008568,A=1.000000)" 2.0 "Cont")
      (Development|PrintText (Utilities|Text|FormatText "Init Dens: {d}" _returnvalue_6) true false "(R=1.000000,G=0.072390,B=0.102237,A=1.000000)" 2.0 "InDens")
      (Development|PrintText (Utilities|Text|FormatText "Fin Dens: {d}" (Class|TerrainShaper|GetFinalDensityatXYZBP _returnvalue_5 _returnvalue_6 (.z _returnvalue_2) (Class|TerrainShaper|GetTerrainHeightatXYBP _returnvalue_5 (.x _returnvalue_2) (.y _returnvalue_2)) (Class|TerrainShaper|GetSFatXYBP _returnvalue_5 (.x _returnvalue_2) (.y _returnvalue_2)))) true false "(R=1.000000,G=0.072390,B=0.102237,A=1.000000)" 2.0 "FDens")
      (Development|PrintText (Utilities|Text|FormatText "Ter H: {h}" (Class|TerrainShaper|GetTerrainHeightatXYBP _returnvalue_5 (.x _returnvalue_3) (.y _returnvalue_3))) true false "(R=1.000000,G=0.072390,B=0.102237,A=1.000000)" 2.0 "TH"))
    (:then_1
      (bind (_bhitsuccesful _hitresult) (Class|PlayerCharacter|VisibilityLineTrace))
      (if _bhitsuccesful
        (Development|PrintString (Utilities|String|Append "Hit Actor: " (Utilities|GetDisplayName (.HitActor (Collision|BreakHitResult _hitresult))) "Hit Material:  " (Utilities|GetDisplayName (Rendering|Material|GetMaterial (.HitComponent (Collision|BreakHitResult _hitresult)) 0))) true false "(R=1.000000,G=0.875294,B=0.049854,A=1.000000)" 2.0 "VisDebug")))))

(fn ShowLocationDebug
  (bind _returnvalue (Transformation|GetActorLocation))
  (bind _returnvalue_2 (Transformation|GetActorLocation))
  (bind _returnvalue_3 (Transformation|GetActorLocation))
  (bind _returnvalue_4 (Transformation|GetActorLocation))
  (bind _returnvalue_5 (Class|ChunkUtilityLib|WorldLocationtoChunkLocationBP _returnvalue_4))
  (bind _returnvalue_6 (Class|ChunkUtilityLib|WorldLocationtoChunkLocationBP _returnvalue))
  (bind _returnvalue_7 (Class|ChunkUtilityLib|WorldLocationtoChunkLocationBP _returnvalue_3))
  (bind _returnvalue_8 (Class|ChunkUtilityLib|GetRegionID _returnvalue_7))
  (bind _returnvalue_9 (Class|ChunkUtilityLib|GetRegionID _returnvalue_6))
  (bind _returnvalue_10 (Class|ChunkUtilityLib|GetRegionOrigin _returnvalue_8))
  (Development|PrintText (Utilities|Text|FormatText "X/Y/Z Loc:  {X} / {Y} / {Z}   
Chunk Loc: {CX} / {CY} / {CZ}  
RegionID: {RX} / {RY} / {RZ}  
RegionOrg: {ROX} /  {ROY} / {ROZ}" (.x _returnvalue_2) (.y _returnvalue_2) (.z _returnvalue_2) (.x _returnvalue_5) (.y _returnvalue_5) (.z _returnvalue_5) (.x _returnvalue_9) (.y _returnvalue_9) (.z _returnvalue_9) (.x _returnvalue_10) (.y _returnvalue_10) (.z _returnvalue_10)) true false "(R=0.985243,G=0.431361,B=1.000000,A=1.000000)" 2.0 "LocDEBUG"))