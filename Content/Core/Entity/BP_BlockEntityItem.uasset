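; Block item entity: an item actor that shows a block and can be picked up into a player's inventory.
; Construction creates a dynamic material for the mesh, setting six per-face texture indices from BlockDataSubsystem by item ID; single-texture blocks use the up texture throughout.
; When a player-tagged character interacts, it adds the item to the PlayerState's inventory component, reduces the stack by the returned amount and destroys itself at zero.
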(fn ConstructionScript
  (|CallParentFunction)
  (CallFunction|ConstrScriptFunc))

(fn OnInteractedwith
  (params (interactedBy :type Base%20Character%20Object%20Reference) (traceResult :type Hit%20Result%20Structure%20%28by%20ref%29))
  (if (GameplayTags|HasTag (Variables|/Script/Terrestre.BaseCharacter|GetCharacterGameplayTags interactedBy) "(TagName=\"Terrestre.Character.Player\")")
    (bind _returnvalue (Class|InventoryComponent|AddItemtoStorage (Actor|GetComponentbyClass (Variables|/Script/Engine.Pawn|GetPlayerState interactedBy) "/Script/Terrestre.InventoryComponent") (Variables|Default|GetBoundItem) -1))
    (if (> _returnvalue 0)
      (bind _output_get (Variables|Default|SetItemCountInThisStack (- (Variables|Default|GetItemCountInThisStack) _returnvalue)))
      (if (== _output_get 0)
        (Actor|DestroyActor))
      (return (Utilities|Struct|MakeInteractionResult self true true))
      (else
        (return (Utilities|Struct|MakeInteractionResult self false false))))))

(fn ConstrScriptFunc
  (bind _returnvalue (|BlockDataSubsystem))
  (bind _bounditem (Variables|Default|GetBoundItem))
  (bind _itemid (Variables|/Script/Terrestre.ItemBase|GetItemID _bounditem))
  (bind _returnvalue_2 (Class|KismetMathLibrary|ToInt64(Integer) _itemid))
  (bind _outdata (Class|BlockDataSubsystem|GetBlockDataBP _returnvalue _returnvalue_2))
  (bind (_displayname _droppeditemid _bhassingletexture _textureindexup _textureindexdown _textureindexleft _textureindexright _textureindexforward _textureindexbackward) (Utilities|Struct|BreakBlockData _outdata))
  (bind _returnvalue_3 (Math|Conversions|ToFloat(Integer) _textureindexup))
  (bind _returnvalue_4 (Rendering|Material|CreateDynamicMaterialInstance "/Game/Core/World/Materials/Items/M_BlockItemEntity.M_BlockItemEntity" "None" "None" :!class /Script/Engine.KismetMaterialLibrary))
  (bind _output_get (Variables|Default|SetMID_Item _returnvalue_4))
  (Rendering|Material|SetScalarParameterValue _output_get "Up Texture Index" _returnvalue_3 :!class /Script/Engine.MaterialInstanceDynamic)
  (Rendering|Material|SetScalarParameterValue (Variables|Default|GetMID_Item) "Down Texture Index" (Math|Float|SelectFloat _returnvalue_3 (Math|Conversions|ToFloat(Integer) _textureindexdown) _bhassingletexture) :!class /Script/Engine.MaterialInstanceDynamic)
  (Rendering|Material|SetScalarParameterValue (Variables|Default|GetMID_Item) "Forward Texture Index" (Math|Float|SelectFloat _returnvalue_3 (Math|Conversions|ToFloat(Integer) _textureindexforward) _bhassingletexture) :!class /Script/Engine.MaterialInstanceDynamic)
  (Rendering|Material|SetScalarParameterValue (Variables|Default|GetMID_Item) "Backward Texture Index" (Math|Float|SelectFloat _returnvalue_3 (Math|Conversions|ToFloat(Integer) _textureindexbackward) _bhassingletexture) :!class /Script/Engine.MaterialInstanceDynamic)
  (Rendering|Material|SetScalarParameterValue (Variables|Default|GetMID_Item) "Left Texture Index" (Math|Float|SelectFloat _returnvalue_3 (Math|Conversions|ToFloat(Integer) _textureindexleft) _bhassingletexture) :!class /Script/Engine.MaterialInstanceDynamic)
  (Rendering|Material|SetScalarParameterValue (Variables|Default|GetMID_Item) "Right Texture Index" (Math|Float|SelectFloat _returnvalue_3 (Math|Conversions|ToFloat(Integer) _textureindexright) _bhassingletexture) :!class /Script/Engine.MaterialInstanceDynamic)
  (Rendering|Material|SetMaterial (Variables|Default|GetItemMesh) 0 (Variables|Default|GetMID_Item)))