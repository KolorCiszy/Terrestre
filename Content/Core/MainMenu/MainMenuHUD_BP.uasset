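; Main menu HUD that spawns the menu widget and drives navigation, singleplayer world management and game launch.
; Button clicks dispatch on type and menu state, with UpdateMenuState toggling panel visibility.
; GameSavingSubsystem lists, creates and deletes worlds, seeding new ones from their name.
; A selection event toggles Play/Delete and sets the world GameInstance loads; Tick prints it for debugging.
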(event Custom|OnButtonClicked
  (params (ButtonType :type EMainMenuButtons%20Enum :default "NewEnumerator0"))
  (bind _selectedspworld (Variables|Default|GetSelectedSPWorld))
  (bind _worldname (Variables|/Script/Terrestre.WorldSaveData|GetWorldName _selectedspworld))
  (switch Utilities|FlowControl|Switch|SwitchonEMainMenuButtons ButtonType
    (:NewEnumerator0
      (CallFunction|UpdateMenuState "NewEnumerator1"))
    (:NewEnumerator1
      (CallFunction|UpdateMenuState "NewEnumerator2"))
    (:NewEnumerator2
      (CallFunction|UpdateMenuState "NewEnumerator4"))
    (:NewEnumerator3
      (Game|QuitGame (Game|Player|GetOwningPlayerController) "Quit" false))
    (:NewEnumerator4
      (switch Utilities|FlowControl|Switch|SwitchonEMainMenuState (Variables|Default|GetMainMenuState)
        (:NewEnumerator1
          (CallFunction|UpdateMenuState "NewEnumerator3"))
        (:NewEnumerator3
          (bind (_bsuccess_ _errormsg) (CallFunction|TryCreateNewWorld (Utilities|String|ToString(Text) (Variables|/Script/UMG.EditableText|GetText (Variables|/Game/Core/MainMenu/WidgetBPs/CreateNewWorld_WBP.CreateNewWorld_WBP_C|GetEnterWorldNameBox (Variables|/Game/Core/MainMenu/WidgetBPs/MainMenu_WBP.MainMenu_WBP_C|GetCreateNewWorld_WBP (Variables|Default|GetMainMenuWidget)))))))
          (if _bsuccess_
            (CallFunction|UpdateMenuState "NewEnumerator1")
            (else
              (Variables|/Script/UMG.TextBlock|SetText (Variables|/Game/Core/MainMenu/WidgetBPs/CreateNewWorld_WBP.CreateNewWorld_WBP_C|GetCreationErrorText (Variables|/Game/Core/MainMenu/WidgetBPs/MainMenu_WBP.MainMenu_WBP_C|GetCreateNewWorld_WBP (Variables|Default|GetMainMenuWidget))) (Utilities|Text|ToText(String) _errormsg)))))))
    (:NewEnumerator5
      (CallFunction|UpdateMenuState (Utilities|Select :Index (Variables|Default|GetMainMenuState) :NewEnumerator0 "NewEnumerator0" :NewEnumerator1 "NewEnumerator0" :NewEnumerator2 "NewEnumerator0" :NewEnumerator3 "NewEnumerator1" :NewEnumerator4 "NewEnumerator0" :NewEnumerator5 "NewEnumerator0")))
    (:NewEnumerator6
      (switch Utilities|FlowControl|Switch|SwitchonEMainMenuState (Variables|Default|GetMainMenuState)
        (:NewEnumerator1
          (if (not (Utilities|Array|IsEmpty _worldname))
            (bind _returnvalue (Class|GameSavingSubsystem|DeleteSavedWorld (Subsystems|GetGameSavingSubsystem) _worldname))
            (if _returnvalue
              (CallFunction|RefreshSPWorlds))))))
    (:NewEnumerator7
      (switch Utilities|FlowControl|Switch|SwitchonEMainMenuState (Variables|Default|GetMainMenuState)
        (:NewEnumerator1
          (if true
            (CallFunction|UpdateMenuState "NewEnumerator5")
            (Utilities|FlowControl|Delay 0.1)
            (Class|TerrestreGameInstance|LoadWorld (.AsTerrestre%20Game%20Instance (Utilities|Casting|CastToTerrestreGameInstance (Game|GetGameInstance))) (Variables|Default|GetSelectedSPWorld))))))))

(event Custom|OnSpWorldSelectionChangedEvent
  (CallFunction|UpdateSelectedSPWorld))

(event EventBeginPlay
  (bind _returnvalue (UserInterface|CreateWidget "/Game/Core/MainMenu/WidgetBPs/MainMenu_WBP.MainMenu_WBP_C" (Game|Player|GetOwningPlayerController)))
  (bind _output_get (Variables|Default|SetMainMenuWidget _returnvalue))
  (UserInterface|Viewport|AddtoViewport _returnvalue 0)
  (Variables|/Script/Engine.PlayerController|SetbShowMouseCursor (Game|Player|GetOwningPlayerController) true)
  (EventDispatchers|AssignOnSpWorldSelectionChanged (delegate Custom|OnSpWorldSelectionChangedEvent)))

(event EventTick
  (params (DeltaSeconds :type Float%20%28single-precision%29))
  (bind _selectedspworld (Variables|Default|GetSelectedSPWorld))
  (Utilities|IsValid _selectedspworld
    (:Is%20Valid
      (Development|PrintString (Utilities|String|Append "Selected world:" (Variables|/Script/Terrestre.WorldSaveData|GetWorldName _selectedspworld) "Seed: " (Utilities|String|ToString(Integer) (Variables|/Script/Terrestre.WorldSaveData|GetWorldSeed _selectedspworld))) true true "(R=1.000000,G=0.266839,B=0.147041,A=1.000000)" 2.0 "SPWorld"))))

(fn ConstructionScript)

(fn RefreshSPWorlds
  (bind _mainmenuwidget (Variables|Default|GetMainMenuWidget))
  (bind _spworldselect_wbp (Variables|/Game/Core/MainMenu/WidgetBPs/MainMenu_WBP.MainMenu_WBP_C|GetSPWorldSelect_WBP _mainmenuwidget))
  (bind _worldlist (Variables|/Game/Core/MainMenu/WidgetBPs/SPWorldSelect_WBP.SPWorldSelect_WBP_C|GetWorldList _spworldselect_wbp))
  (Class|ListView|ClearSelection _worldlist)
  (Class|ListView|SetListItems _worldlist (Class|GameSavingSubsystem|GetSavedWorlds (Subsystems|GetGameSavingSubsystem)))
  (Default|CallOnSpWorldSelectionChanged))

(fn UpdateMenuState
  (params (NewState :type EMainMenuState%20Enum :default "NewEnumerator0"))
  (bind _mainmenuwidget (Variables|Default|GetMainMenuWidget))
  (bind _mainmenuwidget_2 (Variables|Default|GetMainMenuWidget))
  (bind _mainmenuwidget_3 (Variables|Default|GetMainMenuWidget))
  (bind _mainmenuwidget_4 (Variables|Default|GetMainMenuWidget))
  (bind _mainmenuwidget_5 (Variables|Default|GetMainMenuWidget))
  (bind _mainmenuwidget_6 (Variables|Default|GetMainMenuWidget))
  (bind _output_get (Variables|Default|SetMainMenuState NewState))
  (switch Utilities|FlowControl|Switch|SwitchonEMainMenuState _output_get
    (:NewEnumerator0
      (Widget|SetVisibility (Variables|/Game/Core/MainMenu/WidgetBPs/MainMenu_WBP.MainMenu_WBP_C|GetMainMenuButtons _mainmenuwidget) "Visible")
      (Widget|SetVisibility (Variables|/Game/Core/MainMenu/WidgetBPs/MainMenu_WBP.MainMenu_WBP_C|GetCreateNewWorld_WBP _mainmenuwidget) "Collapsed")
      (Widget|SetVisibility (Variables|/Game/Core/MainMenu/WidgetBPs/MainMenu_WBP.MainMenu_WBP_C|GetSPWorldSelect_WBP _mainmenuwidget) "Collapsed")
      (Widget|SetVisibility (Variables|/Game/Core/MainMenu/WidgetBPs/MainMenu_WBP.MainMenu_WBP_C|GetTitle _mainmenuwidget) "Visible")
      (Widget|SetVisibility (Variables|/Game/Core/MainMenu/WidgetBPs/MainMenu_WBP.MainMenu_WBP_C|GetMPServerSelect_WBP _mainmenuwidget) "Collapsed")
      (Widget|SetVisibility (Variables|/Game/Core/MainMenu/WidgetBPs/MainMenu_WBP.MainMenu_WBP_C|GetSettings_WBP _mainmenuwidget) "Collapsed"))
    (:NewEnumerator1
      (Widget|SetVisibility (Variables|/Game/Core/MainMenu/WidgetBPs/MainMenu_WBP.MainMenu_WBP_C|GetSPWorldSelect_WBP _mainmenuwidget_5) "Visible")
      (Widget|SetVisibility (Variables|/Game/Core/MainMenu/WidgetBPs/MainMenu_WBP.MainMenu_WBP_C|GetMainMenuButtons _mainmenuwidget_5) "Collapsed")
      (Widget|SetVisibility (Variables|/Game/Core/MainMenu/WidgetBPs/MainMenu_WBP.MainMenu_WBP_C|GetCreateNewWorld_WBP _mainmenuwidget_5) "Collapsed")
      (Widget|SetVisibility (Variables|/Game/Core/MainMenu/WidgetBPs/MainMenu_WBP.MainMenu_WBP_C|GetTitle _mainmenuwidget_5) "Collapsed")
      (CallFunction|RefreshSPWorlds))
    (:NewEnumerator2
      (Widget|SetVisibility (Variables|/Game/Core/MainMenu/WidgetBPs/MainMenu_WBP.MainMenu_WBP_C|GetMPServerSelect_WBP _mainmenuwidget_6) "Visible")
      (Widget|SetVisibility (Variables|/Game/Core/MainMenu/WidgetBPs/MainMenu_WBP.MainMenu_WBP_C|GetMainMenuButtons _mainmenuwidget_6) "Collapsed")
      (Widget|SetVisibility (Variables|/Game/Core/MainMenu/WidgetBPs/MainMenu_WBP.MainMenu_WBP_C|GetTitle _mainmenuwidget_6) "Collapsed"))
    (:NewEnumerator3
      (Widget|SetVisibility (Variables|/Game/Core/MainMenu/WidgetBPs/MainMenu_WBP.MainMenu_WBP_C|GetCreateNewWorld_WBP _mainmenuwidget_4) "Visible")
      (Widget|SetVisibility (Variables|/Game/Core/MainMenu/WidgetBPs/MainMenu_WBP.MainMenu_WBP_C|GetMainMenuButtons _mainmenuwidget_4) "Collapsed")
      (Widget|SetVisibility (Variables|/Game/Core/MainMenu/WidgetBPs/MainMenu_WBP.MainMenu_WBP_C|GetSPWorldSelect_WBP _mainmenuwidget_4) "Collapsed"))
    (:NewEnumerator4
      (Widget|SetVisibility (Variables|/Game/Core/MainMenu/WidgetBPs/MainMenu_WBP.MainMenu_WBP_C|GetTitle _mainmenuwidget_2) "Collapsed")
      (Widget|SetVisibility (Variables|/Game/Core/MainMenu/WidgetBPs/MainMenu_WBP.MainMenu_WBP_C|GetMainMenuButtons _mainmenuwidget_2) "Collapsed")
      (Widget|SetVisibility (Variables|/Game/Core/MainMenu/WidgetBPs/MainMenu_WBP.MainMenu_WBP_C|GetSettings_WBP _mainmenuwidget_2) "Visible"))
    (:NewEnumerator5
      (Widget|SetVisibility (Variables|/Game/Core/MainMenu/WidgetBPs/MainMenu_WBP.MainMenu_WBP_C|GetSPWorldSelect_WBP _mainmenuwidget_3) "Collapsed")
      (Widget|SetVisibility (Variables|/Game/Core/MainMenu/WidgetBPs/MainMenu_WBP.MainMenu_WBP_C|GetMainMenuButtons _mainmenuwidget_3) "Collapsed")
      (Widget|SetVisibility (Variables|/Game/Core/MainMenu/WidgetBPs/MainMenu_WBP.MainMenu_WBP_C|GetCreateNewWorld_WBP _mainmenuwidget_3) "Collapsed")
      (Widget|SetVisibility (Variables|/Game/Core/MainMenu/WidgetBPs/MainMenu_WBP.MainMenu_WBP_C|GetGameLoading_WBP _mainmenuwidget_3) "Visible"))))

(fn TryCreateNewWorld
  (params (WorldName :type String))
  (if (Class|GameSavingSubsystem|DoesSavedWorldExist (Subsystems|GetGameSavingSubsystem) WorldName)
    (return false "A world with this name already exists.")
    (else
      (bind _returnvalue (Game|ConstructObjectfromClass "/Script/Terrestre.WorldSaveData" WorldName (Class|WorldSaveData|WorldSeedfromString (Utilities|String|ToString(Text) (Variables|/Script/UMG.EditableText|GetText (Variables|/Game/Core/MainMenu/WidgetBPs/CreateNewWorld_WBP.CreateNewWorld_WBP_C|GetEnterWorldNameBox (Variables|/Game/Core/MainMenu/WidgetBPs/MainMenu_WBP.MainMenu_WBP_C|GetCreateNewWorld_WBP (Variables|Default|GetMainMenuWidget)))))) (Math|DateTime|Now) (Math|DateTime|Now)))
      (if true
        (bind _returnvalue_2 (Class|GameSavingSubsystem|SaveWorldData (Subsystems|GetGameSavingSubsystem) _returnvalue))
        (if _returnvalue_2
          (return true "")
          (else
            (return false "Failed to save world to disk.")))
        (else
          (return false "World data is invalid."))))))

(fn UpdateSelectedSPWorld
  (bind _mainmenuwidget (Variables|Default|GetMainMenuWidget))
  (bind _mainmenuwidget_2 (Variables|Default|GetMainMenuWidget))
  (bind _spworldselect_wbp (Variables|/Game/Core/MainMenu/WidgetBPs/MainMenu_WBP.MainMenu_WBP_C|GetSPWorldSelect_WBP _mainmenuwidget))
  (bind _spworldselect_wbp_2 (Variables|/Game/Core/MainMenu/WidgetBPs/MainMenu_WBP.MainMenu_WBP_C|GetSPWorldSelect_WBP _mainmenuwidget_2))
  (bind _asworld_save_data (Utilities|Casting|CastToWorldSaveData (Class|ListView|GetSelectedItem (Variables|/Game/Core/MainMenu/WidgetBPs/SPWorldSelect_WBP.SPWorldSelect_WBP_C|GetWorldList (Variables|/Game/Core/MainMenu/WidgetBPs/MainMenu_WBP.MainMenu_WBP_C|GetSPWorldSelect_WBP (Variables|Default|GetMainMenuWidget)))))
    (:then
      (Variables|Default|SetSelectedSPWorld _asworld_save_data)
      (Widget|SetIsEnabled (Variables|/Game/Core/MainMenu/WidgetBPs/SPWorldSelect_WBP.SPWorldSelect_WBP_C|GetPlayButton _spworldselect_wbp_2) true)
      (Widget|SetIsEnabled (Variables|/Game/Core/MainMenu/WidgetBPs/SPWorldSelect_WBP.SPWorldSelect_WBP_C|GetDeleteButton _spworldselect_wbp_2) true))
    (:CastFailed
      (Variables|Default|SetSelectedSPWorld 0)
      (Widget|SetIsEnabled (Variables|/Game/Core/MainMenu/WidgetBPs/SPWorldSelect_WBP.SPWorldSelect_WBP_C|GetPlayButton _spworldselect_wbp) false)
      (Widget|SetIsEnabled (Variables|/Game/Core/MainMenu/WidgetBPs/SPWorldSelect_WBP.SPWorldSelect_WBP_C|GetDeleteButton _spworldselect_wbp) false))))