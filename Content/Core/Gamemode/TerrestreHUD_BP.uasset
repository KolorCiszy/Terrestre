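; HUD Blueprint that creates the player's main HUD widget and drives its inventory window and hotbar.
; It binds to the player controller's refresh event, handling only the inventory flag, and copies items from the PlayerState's InventoryComponent into backpack slots, mirroring the first ones to the hotbar.
; Separate functions toggle inventory window visibility and move the hotbar selection highlight to the controller's selected slot.
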(event Custom|UpdateHotbarSlots
  (bind _returnvalue (Game|Player|GetOwningPlayerController))
  (bind _hudwidget (Variables|Default|GetHUDWidget))
  (bind _asterrestre_player_controller_bp (Utilities|Casting|CastToTerrestrePlayerController_BP _returnvalue))
  (bind _hotbarslots_wbp (Variables|/Game/Core/UI/Hotbar/HUD_WBP.HUD_WBP_C|GetHotbarSlots_WBP _hudwidget))
  (bind _returnvalue_2 (Class|TerrestrePlayerController|GetSelectedHotbarSlot _asterrestre_player_controller_bp))
  (bind _uiselectedslot (Variables|/Game/Core/UI/Hotbar/HotbarSlots_WBP.HotbarSlots_WBP_C|GetUISelectedSlot _hotbarslots_wbp))
  (Utilities|IsValid _hudwidget
    (:Is%20Valid
      (if (!= _uiselectedslot _returnvalue_2)
        (Class|IHotbarBP|SetSlotSelected(Message) _hotbarslots_wbp _uiselectedslot false)
        (Class|IHotbarBP|SetSlotSelected(Message) _hotbarslots_wbp _returnvalue_2 true)))))

(event Custom|OnRefreshPlayerHUD_Event
  (params (bRefreshHealthBar? :type Boolean) (bRefreshInventory? :type Boolean))
  (if bRefreshInventory?
    (CallFunction|UpdateInventory)))

(event EventBeginPlay
  (bind _returnvalue (UserInterface|CreateWidget "/Game/Core/UI/Hotbar/HUD_WBP.HUD_WBP_C" (Game|Player|GetOwningPlayerController)))
  (bind _output_get (Variables|Default|SetHUDWidget _returnvalue))
  (UserInterface|Viewport|AddtoViewport _output_get 0)
  (EventDispatchers|AssignOnRefreshPlayerHUD (.AsTerrestre%20Player%20Controller%20BP (Utilities|Casting|CastToTerrestrePlayerController_BP (Game|Player|GetOwningPlayerController))) (delegate Custom|OnRefreshPlayerHUD_Event)))

(fn ConstructionScript)

(fn SetInventoryWindowVisibility
  (params (bVisible? :type Boolean))
  (if bVisible?
    (Widget|SetVisibility (Variables|/Game/Core/UI/Hotbar/HUD_WBP.HUD_WBP_C|GetInventoryWindow_WBP (Variables|Default|GetHUDWidget)) "Visible")
    (else
      (Widget|SetVisibility (Variables|/Game/Core/UI/Hotbar/HUD_WBP.HUD_WBP_C|GetInventoryWindow_WBP (Variables|Default|GetHUDWidget)) "Collapsed"))))

(fn UpdateInventory
  (bind _returnvalue (Game|Player|GetOwningPlayerController))
  (bind _playerstate (Variables|/Script/Engine.Controller|GetPlayerState _returnvalue))
  (bind _returnvalue_2 (Actor|GetComponentbyClass _playerstate "/Script/Terrestre.InventoryComponent"))
  (Utilities|IsValid _returnvalue_2
    (:Is%20Valid
      (bind _returnvalue_3 (Class|InventoryComponent|GetStoredItems _returnvalue_2))
      (for (_array_element _array_index) _returnvalue_3
        (Default|UpdateBackpackSlot (Variables|/Game/Core/UI/Hotbar/HUD_WBP.HUD_WBP_C|GetInventoryWindow_WBP (Variables|Default|GetHUDWidget)) _array_index _array_element)
        (if (< _array_index (Default|GetHotbarSlotCount (Variables|Default|GetHUDWidget)))
          (Default|UpdateHotbarSlot (Variables|Default|GetHUDWidget) (Math|Conversions|ToByte(Integer) _array_index) _array_element))))))