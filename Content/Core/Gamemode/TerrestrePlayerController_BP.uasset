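; Player controller for Terrestre that possesses the character and turns Enhanced Input into attacks, block placement, interaction, hotbar selection and inventory display.
; Clicks and interactions send messages to the actor under the character's visibility trace, with attack and placement gated by PlayerState cooldowns.
; Message results drive HUD inventory refreshes; opening the inventory switches to UI-only input.
; Q saves player data, and double-tap toggles flight through console commands.
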(event Input|EnhancedActionEvents|EnhancedInputActionPlayerHotbarSlot_IA
  (params (ActionValue :type Float%20%28double-precision%29) (ElapsedSeconds :type Float%20%28double-precision%29) (TriggeredSeconds :type Float%20%28double-precision%29) (InputAction :type Input%20Action%20Object%20Reference :default "/Game/Core/Player/Input/PlayerHotbarSlot_IA.PlayerHotbarSlot_IA"))
  (bind _returnvalue (Math|Float|Truncate ActionValue))
  (bind _returnvalue_2 (- _returnvalue 1))
  (bind _returnvalue_3 (Math|Integer|%(Integer) _returnvalue_2 10))
  (bind _returnvalue_4 (Math|Conversions|ToByte(Integer) _returnvalue_3))
  (:Started
    (Class|TerrestrePlayerController|SetSelectedHotbarSlot _returnvalue_4)
    (Class|InventoryComponent|SetHeldItem (Variables|/Script/Terrestre.TerrestrePlayerState|GetMainInventory (.AsTerrestre%20Player%20State%20BP (Utilities|Casting|CastToTerrestrePlayerState_BP (Variables|Default|GetPlayerState)))) (Math|Conversions|ToInteger(Byte) _returnvalue_4))))

(event Input|EnhancedActionEvents|EnhancedInputActionPlayerToggleInventory_IA
  (params (ActionValue :type Boolean) (ElapsedSeconds :type Float%20%28double-precision%29) (TriggeredSeconds :type Float%20%28double-precision%29) (InputAction :type Input%20Action%20Object%20Reference :default "/Game/Core/Player/Input/PlayerToggleInventory_IA.PlayerToggleInventory_IA"))
  (bind _returnvalue (HUD|GetHUD))
  (bind _asterrestre_hud_bp (Utilities|Casting|CastToTerrestreHUD_BP _returnvalue))
  (:Started
    (Default|SetInventoryWindowVisibility _asterrestre_hud_bp true)
    (Input|SetInputModeUIOnly self (Variables|/Game/Core/UI/Hotbar/HUD_WBP.HUD_WBP_C|GetInventoryWindow_WBP (Variables|/Game/Core/Gamemode/TerrestreHUD_BP.TerrestreHUD_BP_C|GetHUDWidget _asterrestre_hud_bp)) "DoNotLock" true)
    (Variables|Default|SetbShowMouseCursor true)))

(event Input|EnhancedActionEvents|EnhancedInputActionPlayerLMB_IA
  (params (ActionValue :type Boolean) (ElapsedSeconds :type Float%20%28double-precision%29) (TriggeredSeconds :type Float%20%28double-precision%29) (InputAction :type Input%20Action%20Object%20Reference :default "/Game/Core/Player/Input/PlayerLMB_IA.PlayerLMB_IA"))
  (bind _returnvalue (Pawn|GetControlledPawn))
  (bind _playerstate (Variables|Default|GetPlayerState))
  (bind _asterrestre_player_state_bp (Utilities|Casting|CastToTerrestrePlayerState_BP _playerstate))
  (bind _asplayer_character_bp (Utilities|Casting|CastToPlayerCharacter_BP _returnvalue))
  (bind _returnvalue_2 (Class|PlayerCharacter|GetVisibilityResult _asplayer_character_bp))
  (if (Math|Float|NearlyEqual(Float) (Class|TerrestrePlayerState|GetAttackCooldown _asterrestre_player_state_bp) 0.0 1e-05)
    (Class|TerrestrePlayerState|TriggerAttackCooldown _asterrestre_player_state_bp)
    (bind _returnvalue_3 (Class|InteractableActor|OnLeftMouseButton(Message) (CallFunction|GetHitActor _returnvalue_2) _asplayer_character_bp _returnvalue_2))
    (Default|CallOnRefreshPlayerHUD false (.bShouldRefreshInventoryUI (Utilities|Struct|BreakInteractionResult _returnvalue_3)))))

(event Input|EnhancedActionEvents|EnhancedInputActionPlayerRMB_IA
  (params (ActionValue :type Boolean) (ElapsedSeconds :type Float%20%28double-precision%29) (TriggeredSeconds :type Float%20%28double-precision%29) (InputAction :type Input%20Action%20Object%20Reference :default "/Game/Core/Player/Input/PlayerRMB_IA.PlayerRMB_IA"))
  (bind _returnvalue (Pawn|GetControlledPawn))
  (bind _playerstate (Variables|Default|GetPlayerState))
  (bind _asterrestre_player_state_bp (Utilities|Casting|CastToTerrestrePlayerState_BP _playerstate))
  (bind _asplayer_character_bp (Utilities|Casting|CastToPlayerCharacter_BP _returnvalue))
  (bind _returnvalue_2 (Class|PlayerCharacter|GetVisibilityResult _asplayer_character_bp))
  (if (Math|Float|NearlyEqual(Float) (Class|TerrestrePlayerState|GetBlockPlaceCooldown _asterrestre_player_state_bp) 0.0 1e-05)
    (bind _returnvalue_3 (Class|InteractableActor|OnRightMouseButton(Message) (CallFunction|GetHitActor _returnvalue_2) _asplayer_character_bp _returnvalue_2))
    (if (.bSuccess (Utilities|Struct|BreakInteractionResult _returnvalue_3))
      (Class|TerrestrePlayerState|TriggerBlockPlaceCooldown _asterrestre_player_state_bp)
      (Default|CallOnRefreshPlayerHUD false (.bShouldRefreshInventoryUI (Utilities|Struct|BreakInteractionResult _returnvalue_3))))))

(event Input|EnhancedActionEvents|EnhancedInputActionPlayerInteract_IA
  (params (ActionValue :type Boolean) (ElapsedSeconds :type Float%20%28double-precision%29) (TriggeredSeconds :type Float%20%28double-precision%29) (InputAction :type Input%20Action%20Object%20Reference :default "/Game/Core/Player/Input/PlayerInteract_IA.PlayerInteract_IA"))
  (bind _returnvalue (Pawn|GetControlledPawn))
  (bind _asplayer_character_bp (Utilities|Casting|CastToPlayerCharacter_BP _returnvalue))
  (bind _returnvalue_2 (Class|PlayerCharacter|GetVisibilityResult _asplayer_character_bp))
  (:Started
    (bind _returnvalue_3 (Class|InteractableActor|OnInteractedwith(Message) (CallFunction|GetHitActor _returnvalue_2) _asplayer_character_bp _returnvalue_2))
    (Default|CallOnRefreshPlayerHUD false (.bShouldRefreshInventoryUI (Utilities|Struct|BreakInteractionResult _returnvalue_3)))))

(event Input|EnhancedActionEvents|EnhancedInputActionPlayerTriggerFlight_IA
  (params (ActionValue :type Boolean) (ElapsedSeconds :type Float%20%28double-precision%29) (TriggeredSeconds :type Float%20%28double-precision%29) (InputAction :type Input%20Action%20Object%20Reference :default "/Game/PlayerTriggerFlight_IA.PlayerTriggerFlight_IA"))
  (:Started
    (if (Variables|Default|GetbTriggerFlightNextInput)
      (if (Class|NavMovementComponent|IsFlying (Variables|/Script/Engine.Character|GetCharacterMovement (.AsCharacter (Utilities|Casting|CastToCharacter (Pawn|GetControlledPawn)))))
        (Development|ExecuteConsoleCommand "walk" self)
        (else
          (Development|ExecuteConsoleCommand "fly" self)))
      (Variables|Default|SetbTriggerFlightNextInput true)
      (else
        (Variables|Default|SetbTriggerFlightNextInput true)
        (Utilities|FlowControl|Delay 0.2)
        (Variables|Default|SetbTriggerFlightNextInput false)))))

(event EventBeginPlay
  (Pawn|Possess (Game|GetPlayerCharacter 0))
  (Input|SetInputModeGameOnly self false))

(event EventOnUpdateHotbarWidget
  (Default|UpdateHotbarSlots (.AsTerrestre%20HUD%20BP (Utilities|Casting|CastToTerrestreHUD_BP (HUD|GetHUD)))))

(event Input|KeyboardEvents|Q
  (params (Key :type Key%20Structure :default "None"))
  (:Pressed
    (Class|GameSavingSubsystem|SavePlayerData (Subsystems|GetGameSavingSubsystem) (.AsTerrestre%20Player%20State%20BP (Utilities|Casting|CastToTerrestrePlayerState_BP (Variables|Default|GetPlayerState))))))

(fn ConstructionScript)

(fn GetHitActor
  (params (Hit :type Hit%20Result%20Structure%20%28by%20ref%29))
  (return (.HitActor (Collision|BreakHitResult Hit))))