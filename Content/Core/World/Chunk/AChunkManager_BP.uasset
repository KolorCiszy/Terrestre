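; AChunkManager_BP is a chunk manager Blueprint with no active logic of its own, as BeginPlay and the construction script are empty.
; An unconnected, never-executed chain in the event graph would spawn an ExponentialHeightFog with dense, tinted volumetric fog.
; That chain scales the fog's start and volumetric distances from RenderDistance on TerrestreGameMode_BP.
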(event EventBeginPlay)

(fn ConstructionScript)